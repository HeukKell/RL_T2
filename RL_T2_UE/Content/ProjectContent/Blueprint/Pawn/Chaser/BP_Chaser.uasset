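; BP_Chaser is the chaser pawn, which maps shared memory for its lifetime and can rotate in either direction.
; BeginPlay maps the memory and quits the game on failure, and EndPlay unmaps it.
; Rotate_CW and Rotate_CCW events pass +1 or -1 to Rotate, which is defined outside these graphs.
; An unconnected debug chain would display the floored direction angle to the Runner via CheckTargetDir.
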(event `self.ReceiveEndPlay`
  (params (EndPlayReason :type "EEndPlayReason Enum" :default "Destroyed"))
  (`self.UnmapSharedMemory`))

(event `self.ReceiveBeginPlay`
  (bind _returnvalue (`self.MapSharedMemory`))
  (if (not _returnvalue)
    (`KismetSystemLibrary.QuitGame` null "Quit")))

(event `self.ReceiveTick`
  (params (DeltaSeconds :type "Float (single-precision)")))

(event `Rotate_CW`
  (`self.Rotate` 1))

(event `Rotate_CCW`
  (`self.Rotate` -1))

(fn `UserConstructionScript`)