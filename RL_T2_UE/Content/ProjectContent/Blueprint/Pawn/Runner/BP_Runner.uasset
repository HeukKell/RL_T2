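; Runner pawn that moves under AI control to a position computed relative to a Chaser actor, likely to flee it.
; Run and Exec_Run share one path: FindPosition picks a point around the Chaser, then the AIController moves there.
; Find is a debug routine that samples FindPosition repeatedly and draws successful results as points at zero height.
; The move-completed binding is unwired, and Tick and BeginPlay are empty.
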(event `self.ReceiveBeginPlay`)

(event `OnBind_MoveCompleted`
  (params (RequestID :type "AIRequestID Structure") (Result :type "EPathFollowingResult Enum" :default "Success"))
  (switch `EPathFollowingResult` Result
    (:`Success`
      (`KismetSystemLibrary.PrintString` "Moved!"))))

(event `Exec_Run`
  (bind `_asai_컨트롤러` (cast `AIController` (`self.GetController`) :!label _label))
  (bind (_position _returnvalue) (`self.FindPosition` (`self.Chaser`) 500.0))
  (if _returnvalue
    (`AIController.MoveToLocation` `_asai_컨트롤러` _position 5.0 true true false true null true)))

(event `self.Run`
  (goto _label))

(event `Find`
  (for _ (range 201)
    (bind (_position _returnvalue) (`self.FindPosition` (`self.Chaser`) (`KismetMathLibrary.Conv_IntToDouble` 300)))
    (if _returnvalue
      (`KismetSystemLibrary.DrawDebugPoint` (`KismetMathLibrary.MakeVector` (.x _position) (.y _position)) 5.0 (struct :`R` 1.0 :`A` 1.0) 20.0))))

(fn `UserConstructionScript`)

(fn `새 함수`)